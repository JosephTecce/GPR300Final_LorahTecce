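; DropOffPoint_BP is the goal where the player delivers collected humans, with a text counter showing how many remain.
; It counts Human_BP actors at BeginPlay and registers itself on the player character.
; Player overlap deducts and resets the carried count, switching the player to defending once none remain.
; While a RunnerEnemy_BP overlaps, Tick uses a one-second Delay to repeatedly send that runner a player-collision message, damaging the player remotely.
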(event `self.ReceiveBeginPlay`
  (bind _outactors (`GameplayStatics.GetAllActorsOfClass` "/Game/Blueprints/Goal_BP/Human_BP.Human_BP_C"))
  (bind _output_get (set `self.HumansLeft` (`KismetArrayLibrary.Array_Length` _outactors)))
  (`TextRenderComponent.K2_SetText` (`self.Conter#`) (`KismetTextLibrary.Conv_IntToText` _output_get))
  (bind _asfirst_person_character (cast `/Game/FirstPersonBP/Blueprints/FirstPersonCharacter` (`GameplayStatics.GetPlayerCharacter` 0)))
  (set `/Game/FirstPersonBP/Blueprints/FirstPersonCharacter.DropOffPointRef` self _asfirst_person_character))

(event `self.ReceiveActorBeginOverlap`
  (params (OtherActor :type "Actor Object Reference"))
  (bind _asfirst_person_character (cast `/Game/FirstPersonBP/Blueprints/FirstPersonCharacter` OtherActor)
    (:`then`
      (set `self.HumansLeft` (- (`self.HumansLeft`) (`/Game/FirstPersonBP/Blueprints/FirstPersonCharacter.HumansCollected` _asfirst_person_character)))
      (set `/Game/FirstPersonBP/Blueprints/FirstPersonCharacter.HumansCollected` 0 _asfirst_person_character)
      (`self.UpdateCounter`)
      (if (<= (`self.HumansLeft`) 0)
        (bind _asfirst_person_character_2 (cast `/Game/FirstPersonBP/Blueprints/FirstPersonCharacter` (`GameplayStatics.GetPlayerCharacter` 0)))
        (set `/Game/FirstPersonBP/Blueprints/FirstPersonCharacter.IsDefending` true _asfirst_person_character_2)))
    (:`CastFailed`
      (bind _asrunner_enemy_bp (cast `/Game/Blueprints/Enemy_BP/BasicRunner/RunnerEnemy_BP` OtherActor))
      (set `self.DamagePlayer` true)
      (set `self.CurrentRunner` _asrunner_enemy_bp))))

(event `self.ReceiveActorEndOverlap`
  (params (OtherActor :type "Actor Object Reference"))
  (cast `/Game/Blueprints/Enemy_BP/BasicRunner/RunnerEnemy_BP` OtherActor)
  (set `self.DamagePlayer` false)
  (set `self.CurrentRunner` null))

(event `self.ReceiveTick`
  (params (DeltaSeconds :type "Float (single-precision)"))
  (if (`self.DamagePlayer`)
    (`KismetSystemLibrary.Delay` 1.0)
    (bind _asfirst_person_character (cast `/Game/FirstPersonBP/Blueprints/FirstPersonCharacter` (`GameplayStatics.GetPlayerCharacter` 0)))
    (message `/Game/Blueprints/Player_BP/PlayerCollide_Inter.CollidedWithPlayer` (`self.CurrentRunner`) _asfirst_person_character)))

(fn `UpdateCounter`
  (`TextRenderComponent.K2_SetText` (`self.Conter#`) (`KismetTextLibrary.Conv_IntToText` (`self.HumansLeft`))))

(fn `UserConstructionScript`)