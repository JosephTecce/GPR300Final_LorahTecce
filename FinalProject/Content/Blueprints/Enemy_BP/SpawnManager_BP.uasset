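; SpawnManager_BP is a wave manager that spawns runner enemies in growing waves.
; Each tick it gathers all RunnerEnemy_BP actors and adds a fixed, frame-dependent step to a timer, triggering a wave when none remain or the timer passes TimeTillNextAutomaticWave.
; Each wave raises the spawn count, then loops SpawnEnemies to create runners with BasicRunner_BT at random SpawnPoints.
; The random index range includes the array length, one past the last element.
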(event `self.ReceiveBeginPlay`
  (`KismetSystemLibrary.Delay` 5.0)
  (set `self.NoRunnersAlive` true))

(event `self.ReceiveTick`
  (params (DeltaSeconds :type "Float (single-precision)"))
  (bind _outactors (`GameplayStatics.GetAllActorsOfClass` "/Game/Blueprints/Enemy_BP/BasicRunner/RunnerEnemy_BP.RunnerEnemy_BP_C"))
  (bind _output_get (set `self.RunnerLists` _outactors))
  (bind _output_get_2 (set `self.CurrentTime` (+ (`self.CurrentTime`) 0.1)))
  (if (or (<= (`KismetArrayLibrary.Array_Length` _output_get) 0) (> _output_get_2 (`self.TimeTillNextAutomaticWave`)))
    (`self.SpawnNextWave`)
    (set `self.CurrentTime` 0.0)
    (else
      (`KismetSystemLibrary.Delay` 2.0))))

(event `SpawnNextWave`
  (bind _output_get (set `self.AmountToSpawn` (+ (`self.AmountToSpawn`) 5)))
  (for _ (range (+ _output_get 1))
    (`self.SpawnEnemies`)
    (`KismetSystemLibrary.Delay` 0.5)))

(fn `SpawnEnemies`
  (bind _spawnpoints (`self.SpawnPoints`))
  (`AIBlueprintHelperLibrary.SpawnAIFromClass` "/Game/Blueprints/Enemy_BP/BasicRunner/RunnerEnemy_BP.RunnerEnemy_BP_C" "/Game/Blueprints/Enemy_BP/BasicRunner/BasicRunner_BT.BasicRunner_BT" (`self.K2_GetActorLocation` (`|GetArrayItem` _spawnpoints (`KismetMathLibrary.RandomIntegerInRange` 0 (`KismetArrayLibrary.Array_Length` _spawnpoints)))) (struct) false null))

(fn `UserConstructionScript`)