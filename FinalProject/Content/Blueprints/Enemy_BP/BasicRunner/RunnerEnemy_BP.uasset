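; Runner enemy actor that damages the player on collision, takes shot damage and can drop pickups on death.
; Hits notify actors implementing RunnerCollide_Inst, while player collision applies damage only if not invincible, then sets invincibility.
; A lethal shot hides the mesh, disables capsule collision, may spawn ammo or health, and destroys the actor after a delay.
; Death splatter particle collisions spawn randomly sized decals with a random material frame.
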(event `self.ReceiveBeginPlay`
  (set `self.CurrentHealth` (`self.MaxHealth`))
  (set `self.RunnerMesh` (`self.Mesh`)))

(event `/Game/Blueprints/Player_BP/PlayerCollide_Inter.CollidedWithPlayer`
  (params (Player :type "/Game/FirstPersonBP/Blueprints/FirstPersonCharacter Object Reference"))
  (if (not (`/Game/FirstPersonBP/Blueprints/FirstPersonCharacter.IsInvinsible` Player))
    (set `/Game/FirstPersonBP/Blueprints/FirstPersonCharacter.CurHealth` (- (`/Game/FirstPersonBP/Blueprints/FirstPersonCharacter.CurHealth` Player) (`self.Damage`)) Player)
    (set `/Game/FirstPersonBP/Blueprints/FirstPersonCharacter.IsInvinsible` true Player)
    (`/Game/FirstPersonBP/Blueprints/FirstPersonCharacter.DamageEffect` Player)))

(event `self.ReceiveHit`
  (params (MyComp :type "PrimitiveComponent Object Reference") (Other :type "Actor Object Reference") (OtherComp :type "PrimitiveComponent Object Reference") (bSelfMoved :type Boolean) (HitLocation :type "Vector Structure") (HitNormal :type "Vector Structure") (NormalImpulse :type "Vector Structure") (Hit :type "HitResult Structure (by ref)"))
  (if (`KismetSystemLibrary.DoesImplementInterface` Other "/Game/Blueprints/Enemy_BP/BasicRunner/RunnerCollide_Inst.RunnerCollide_Inst_C")
    (message `/Game/Blueprints/Enemy_BP/BasicRunner/RunnerCollide_Inst.CollidedWithRunner` Other self)))

(event `TookDamage`
  (if (<= (`self.CurrentHealth`) 0.0)
    (`self.K2_DestroyActor`)))

(event `RunnerShot`
  (params (TakenDamage :type "Float (double-precision)"))
  (bind _output_get (set `self.CurrentHealth` (- (`self.CurrentHealth`) TakenDamage)))
  (if (<= _output_get 0.0)
    (bind _returnvalue (`GameplayStatics.SpawnEmitterAtLocation` "/Game/Art/Particles/BloodSplatter/DeathSplatter_P.DeathSplatter_P" (`self.K2_GetActorLocation`)))
    (add `ParticleSystemComponent.OnParticleCollide` _returnvalue (delegate `SplatterDecalSpawn`))
    (`PrimitiveComponent.SetCollisionEnabled` (`self.CapsuleComponent`) "NoCollision")
    (`SceneComponent.SetVisibility` (`self.Mesh`) false false)
    (`self.DropItemChance`)
    (`KismetSystemLibrary.Delay` 1.0)
    (`self.K2_DestroyActor`)))

(event `SplatterDecalSpawn`
  (params (EventName :type Name) (EmitterTime :type "Float (double-precision)") (ParticleTime :type Integer) (Location :type "Vector Structure") (Velocity :type "Vector Structure") (Direction :type "Vector Structure") (Normal :type "Vector Structure") (BoneName :type Name) (PhysMat :type "PhysicalMaterial Object Reference"))
  (bind _returnvalue (`KismetMaterialLibrary.CreateDynamicMaterialInstance` "/Game/Art/Particles/BloodSplatter/SplatterDecal_M.SplatterDecal_M"))
  (`MaterialInstanceDynamic.SetScalarParameterValue` _returnvalue "Frame" (`KismetMathLibrary.Conv_IntToDouble` (`KismetMathLibrary.RandomInteger` 11)))
  (`GameplayStatics.SpawnDecalAtLocation` _returnvalue (`KismetMathLibrary.Conv_DoubleToVector` (`KismetMathLibrary.RandomFloatInRange` 20.0 50.0)) Location (`KismetMathLibrary.Conv_VectorToRotator` Normal) 20.0))

(fn `DropItemChance`
  (bind _returnvalue (`self.K2_GetActorLocation`))
  (if (< (`self.DropChance`) (`KismetMathLibrary.RandomIntegerInRange` 1 100))
    (if (`KismetMathLibrary.RandomBool`)
      (`|SpawnActorFromClass` "/Game/Blueprints/Support_BP/AmmoPack_BP.AmmoPack_BP_C" (`KismetMathLibrary.MakeTransform` _returnvalue) "Undefined" "OverrideRootScale" null null)
      (else
        (`|SpawnActorFromClass` "/Game/Blueprints/Support_BP/HealthPack_BP.HealthPack_BP_C" (`KismetMathLibrary.MakeTransform` _returnvalue) "Undefined" "OverrideRootScale" null null)))))

(fn `UserConstructionScript`)