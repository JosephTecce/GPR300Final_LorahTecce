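; A health pickup actor that heals the first-person player character on touch.
; It spins each tick around its yaw axis at a configurable speed.
; When the character overlaps its sphere while below max health, it adds a fixed amount of health clamped to the maximum, then destroys itself, so it stays in place for players at full health.
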(event `self.ReceiveTick`
  (params (DeltaSeconds :type "Float (single-precision)"))
  (`self.K2_AddActorLocalRotation` (`KismetMathLibrary.MakeRotator` 0.0 0.0 (`self.SpinSpeed`))))

(event `self.Sphere.OnComponentBeginOverlap`
  (params (OverlappedComponent :type "PrimitiveComponent Object Reference") (OtherActor :type "Actor Object Reference") (OtherComp :type "PrimitiveComponent Object Reference") (OtherBodyIndex :type Integer) (bFromSweep :type Boolean) (SweepResult :type "HitResult Structure (by ref)"))
  (bind _asfirst_person_character (cast `/Game/FirstPersonBP/Blueprints/FirstPersonCharacter` OtherActor))
  (if (< (`/Game/FirstPersonBP/Blueprints/FirstPersonCharacter.CurHealth` _asfirst_person_character) (`/Game/FirstPersonBP/Blueprints/FirstPersonCharacter.MaxHealth` _asfirst_person_character))
    (set `/Game/FirstPersonBP/Blueprints/FirstPersonCharacter.CurHealth` (`KismetMathLibrary.FClamp` (+ (`/Game/FirstPersonBP/Blueprints/FirstPersonCharacter.CurHealth` _asfirst_person_character) 100.0) 0.0 (`/Game/FirstPersonBP/Blueprints/FirstPersonCharacter.MaxHealth` _asfirst_person_character)) _asfirst_person_character)
    (`self.K2_DestroyActor`)))

(fn `UserConstructionScript`)