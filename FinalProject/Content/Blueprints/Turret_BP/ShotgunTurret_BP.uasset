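; Shotgun turret that fires a spread of ShotgunBullet_BP pellets from its left barrel, extending a parent turret class.
; FireTurret records the fire time, then spawns NumBullets at the FirePosition socket and plays the left recoil timeline.
; RandPointInCircle scatters points in a disc at BulletDistance, sized by the tangent of BulletAngle.
; Each pellet's rotation comes from that point's world-position vector, without subtracting the muzzle location.
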(event `self.ReceiveBeginPlay`
  (`parent.ReceiveBeginPlay`)
  (set `self.BulletAngle` (`self.StartingBulletAngle`)))

(event `self.ReceiveTick`
  (params (DeltaSeconds :type "Float (single-precision)"))
  (`parent.ReceiveTick` DeltaSeconds))

(event `self.FireTurret`
  (bind _barrelleft (`self.BarrelLeft`))
  (bind (_returnvalue_location _returnvalue_rotation _returnvalue_scale) (`KismetMathLibrary.BreakTransform` (`SceneComponent.GetSocketTransform` _barrelleft "FirePosition" "RTS_World")))
  (set `self.TimeOfLastFire` (`KismetSystemLibrary.GetGameTimeInSeconds`))
  (`|ExecutionSequence`
    (:`then_0`
      (goto _label :!via `Reset`))
    (:`then_1`
      (`/Engine/EditorBlueprintResources/StandardMacros.Do N` 1 :!label _label ; Number of times to do something used to set amount of bullets fired form turret
        (:`Exit`
          (for _ (range 1 (+ (`self.NumBullets`) 1))
            (bind _targetpoint (`self.RandPointInCircle` (* (`KismetMathLibrary.DegTan` (`self.BulletAngle`)) (`self.BulletDistance`))))
            (bind (_x _y) (`KismetMathLibrary.BreakVector2D` _targetpoint))
            (`|SpawnActorFromClass` "/Game/Blueprints/Turret_BP/Bullets_BP/ShotgunBullet_BP.ShotgunBullet_BP_C" (`KismetMathLibrary.MakeTransform` _returnvalue_location (`KismetMathLibrary.Conv_VectorToRotator` (+ (+ (`SceneComponent.K2_GetComponentLocation` _barrelleft) (* (`SceneComponent.GetForwardVector` _barrelleft) (`self.BulletDistance`))) (* (`SceneComponent.GetRightVector` _barrelleft) _x) (* (`SceneComponent.GetUpVector` _barrelleft) _y))) _returnvalue_scale) "Undefined" "OverrideRootScale" null null)
            (`TimelineComponent.PlayFromStart` (`self.RecoilTimelineLeft`))))))))

(fn `RandPointInCircle`
  (params (Radius :type "Float (double-precision)"))
  (returns (TargetPoint :type "Vector2D Structure"))
  (locals (Angle :type "Float (double-precision)") (DistFromCenter :type "Float (double-precision)"))
  (set `local.Angle` (`KismetMathLibrary.RandomFloatInRange` 0.0 360.0))
  (set `local.DistFromCenter` (`KismetMathLibrary.RandomFloatInRange` 0.0 (`local.Radius`)))
  (return (`KismetMathLibrary.MakeVector2D` (* (`local.DistFromCenter`) (`KismetMathLibrary.DegCos` (`local.Angle`))) (* (`local.DistFromCenter`) (`KismetMathLibrary.DegSin` (`local.Angle`))))))

(fn `UserConstructionScript`
  (`parent.UserConstructionScript`))