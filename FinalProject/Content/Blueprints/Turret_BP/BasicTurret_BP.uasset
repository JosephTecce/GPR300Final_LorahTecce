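; Auto-turret actor that targets visible pawns within range, ignoring the first player's character, and fires bullets from two barrels.
; Each tick it picks a target by sphere overlap and line of sight, though the closest distance never updates, so the last visible pawn wins.
; The top turns at constant speed with clamped pitch.
; Once cooled down and aligned, a DoN loop fires left then right, with curve-driven timeline recoil.
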(event `self.ReceiveBeginPlay`
  (`TimelineComponent.SetFloatCurve` (`self.RecoilTimelineLeft`) "/Game/Blueprints/Turret_BP/RecoilCurve.RecoilCurve" "Recoil")
  (`TimelineComponent.SetFloatCurve` (`self.RecoilTimelineRight`) "/Game/Blueprints/Turret_BP/RecoilCurve.RecoilCurve" "Recoil"))

(event `self.ReceiveTick`
  (params (DeltaSeconds :type "Float (single-precision)"))
  (`self.FindClosestTarget`)
  (`self.Target`
    (:`then`
      (`self.UpdateTurretRotation` DeltaSeconds)
      (`self.FireUpdate`))
    (:`else`)))

(event `FireTurret`
  (set `self.TimeOfLastFire` (`KismetSystemLibrary.GetGameTimeInSeconds`))
  (`|ExecutionSequence`
    (:`then_0`
      (goto _label :!via `Reset`))
    (:`then_1`
      (`/Engine/EditorBlueprintResources/StandardMacros.Do N` 1 :!label _label ; Number of times to do something used to set amount of bullets fired form turret
        (:`Exit`
          (`|SpawnActorFromClass` "/Game/Blueprints/Turret_BP/Bullets_BP/BasicBullet_BP.BasicBullet_BP_C" (`SceneComponent.GetSocketTransform` (`self.BarrelLeft`) "FirePosition" "RTS_World") "Undefined" "OverrideRootScale" null null) ; Set Bullet Here
          (`TimelineComponent.PlayFromStart` (`self.RecoilTimelineLeft`))
          (`KismetSystemLibrary.Delay` 0.2)
          (`|SpawnActorFromClass` "/Game/Blueprints/Turret_BP/Bullets_BP/BasicBullet_BP.BasicBullet_BP_C" (`SceneComponent.GetSocketTransform` (`self.RightBarrel`) "FirePosition" "RTS_World") "Undefined" "OverrideRootScale" null null) ; Set Bullet Here
          (`TimelineComponent.PlayFromStart` (`self.RecoilTimelineRight`))
          (`KismetSystemLibrary.Delay` 0.2)
          (goto _label))))))

(fn `FindClosestTarget`
  (locals (ClosestDistance_Local :type "Float (double-precision)") (CurDistance_Local :type "Float (double-precision)") (ClosestTarget_Local :type "Actor Object Reference") (CurTarget_Local :type "Actor Object Reference"))
  (set `local.ClosestDistance_Local` (+ (`self.MaxDistance`) 1.0))
  (bind _outactors (`KismetSystemLibrary.SphereOverlapActors` (`self.K2_GetActorLocation`) (`self.MaxDistance`) (`|MakeArray` "ObjectTypeQuery3" :!type "EObjectTypeQuery Enum") "/Script/Engine.Actor" (`|MakeArray` (`GameplayStatics.GetPlayerCharacter` 0) :!type "Actor Object Reference"))) ; Finding Designated Targets
  (for _array_element _outactors
    (bind _output_get (set `local.CurTarget_Local` _array_element))
    (bind _output_get_2 (set `local.CurDistance_Local` (`self.GetDistanceTo` _output_get self)))
    (if (or (< _output_get_2 (`local.ClosestDistance_Local`)) (not (`KismetSystemLibrary.IsValid` (`local.ClosestTarget_Local`))))
      (bind _result (`/Game/Blueprints/FunctionLibrary/BasicFunctionLibrary.HasLineOfSight` (`SceneComponent.K2_GetComponentLocation` (`self.TurretTop`)) (`self.K2_GetActorLocation` (`local.CurTarget_Local`)) (`|MakeArray` self (`local.CurTarget_Local`) :!type "Actor Object Reference")))
      (if _result
        (set `local.ClosestTarget_Local` (`local.CurTarget_Local`))
        (set `local.ClosestDistance_Local` (`local.ClosestDistance_Local`)))))
  (set `self.Target` (`local.ClosestTarget_Local`)) ; Setting Closest Target
)

(fn `FireUpdate`
  (if (> (- (`KismetSystemLibrary.GetGameTimeInSeconds`) (`self.TimeOfLastFire`)) (`self.RateOfFire`))
    (if (> (`KismetMathLibrary.Dot_VectorVector` (`KismetMathLibrary.GetDirectionUnitVector` (`SceneComponent.K2_GetComponentLocation` (`self.TurretTop`)) (`self.K2_GetActorLocation` (`self.Target`))) (`SceneComponent.GetForwardVector` (`self.TurretTop`))) 0.99)
      (`self.FireTurret`))))

(fn `UpdateTurretRotation`
  (params (DeltaSeconds :type "Float (double-precision)"))
  (locals (RotationPoint_Local :type "Rotator Structure" :default (struct)))
  (bind _output_get (set `local.RotationPoint_Local` (`KismetMathLibrary.RInterpTo_Constant` (`SceneComponent.K2_GetComponentRotation` (`self.TurretTop`)) (`KismetMathLibrary.FindLookAtRotation` (`SceneComponent.K2_GetComponentLocation` (`self.TurretTop`)) (`self.K2_GetActorLocation` (`self.Target`))) (`local.DeltaSeconds`) (`self.RotationSpeed`)))) ; Final Output
  (`SceneComponent.K2_SetWorldRotation` (`self.TurretTop`) (`KismetMathLibrary.MakeRotator` (.roll _output_get) (`KismetMathLibrary.ClampAngle` (.pitch _output_get) -45.0 75.0) (.yaw _output_get)) false false))

(fn `UserConstructionScript`)