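; Player component that lets the first-person character vault onto ledges and shows a prompt widget while a vault is possible.
; While idle, Tick traces down ahead of the player, validates ledge height, walkable slope and capsule clearance, then caches the landing point.
; The Vault event switches state, and Tick lerps the player to that point by teleporting without sweep.
; VaultSpeed acts as the move's duration in seconds.
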(event `self.ReceiveBeginPlay`
  (bind _asfirst_person_character (cast `/Game/FirstPersonBP/Blueprints/FirstPersonCharacter` (`self.GetOwner`)))
  (set `self.Player` _asfirst_person_character)
  (bind _returnvalue (`|CreateWidget` "/Game/UI/ValtWidgit.ValtWidgit_C" (cast `PlayerController` (`Pawn.GetController` (`self.Player`)) :!pure true)))
  (set `self.VaultWidget` _returnvalue))

(event `self.ReceiveTick`
  (params (DeltaSeconds :type "Float (single-precision)"))
  (`self.ValtSwitchStateCheck`
    (:`NotVaulting`
      (bind (_result _endlocation) (`self.CanVault`))
      (if _result
        (set `self.EndPosition` _endlocation)
        (if (not (`Widget.IsInViewport` (`self.VaultWidget`)))
          (`UserWidget.AddToViewport` (`self.VaultWidget`) 0))
        (elif (`Widget.IsInViewport` (`self.VaultWidget`))
          (`Widget.RemoveFromParent` (`self.VaultWidget`)))))
    (:`Vaulting`
      (`self.Tick Vault` DeltaSeconds))))

(event `Vault`
  (set `self.VaultProgress` 0.0)
  (set `self.StartPosition` (`Actor.K2_GetActorLocation` (`self.Player`)))
  (set `self.VaultState` "NewEnumerator2"))

(fn `CanVault`
  (returns (Result :type Boolean) (EndLocation :type "Vector Structure"))
  (locals (PlayerCapsule_Local :type "CapsuleComponent Object Reference"))
  (bind _player (`self.Player`))
  (bind _returnvalue (`CapsuleComponent.GetScaledCapsuleHalfHeight` (`local.PlayerCapsule_Local`)))
  (bind _returnvalue_2 (+ (`Actor.K2_GetActorLocation` _player) (* (`Actor.GetActorForwardVector` _player) 70.0)))
  (if (`|EnumEquality` (`self.VaultState`) "NewEnumerator0")
    (set `local.PlayerCapsule_Local` (`Character.CapsuleComponent` (`self.Player`)))
    (bind (_outhit _returnvalue_3) (`KismetSystemLibrary.LineTraceSingle` (+ _returnvalue_2 (`KismetMathLibrary.MakeVector` 0.0 0.0 _returnvalue)) (- _returnvalue_2 (`KismetMathLibrary.MakeVector` 0.0 0.0 _returnvalue)) "TraceTypeQuery1" false (`|MakeArray` (`self.Player`) :!type "Actor Object Reference"))) ; Checking Vault location with linetrace downwards
    (if _returnvalue_3
      (bind (_resault _end_position) (`self.CanVaultToHit` (`local.PlayerCapsule_Local`) _outhit))
      (return _resault _end_position)
      (else
        (return false (0.0 0.0 0.0))))
    (else
      (return false (0.0 0.0 0.0)))))

(fn `CanVaultToHit`
  (params (Capsule :type "CapsuleComponent Object Reference") (Hit :type "HitResult Structure"))
  (returns (Resault :type Boolean) (`End Position` :type "Vector Structure"))
  (locals (EndPosition_Local :type "Vector Structure" :default (0.0 0.0 0.0)))
  (bind (_hit_bblockinghit _hit_binitialoverlap _hit_time _hit_distance _hit_location) (`GameplayStatics.BreakHitResult` (`local.Hit`)))
  (bind (_hit_bblockinghit_2 _hit_binitialoverlap_2 _hit_time_2 _hit_distance_2 _hit_location_2 _hit_impactpoint _hit_normal _hit_impactnormal _hit_physmat _hit_hitactor _hit_hitcomponent _hit_hitbonename _hit_hititem _hit_faceindex _hit_tracestart _hit_traceend) (`GameplayStatics.BreakHitResult` (`local.Hit`)))
  (bind (_hit_bblockinghit_3 _hit_binitialoverlap_3 _hit_time_3 _hit_distance_3 _hit_location_3 _hit_impactpoint_2 _hit_normal_2) (`GameplayStatics.BreakHitResult` (`local.Hit`)))
  (bind _capsule (`local.Capsule`))
  (bind _returnvalue (`CapsuleComponent.GetScaledCapsuleRadius` _capsule))
  (`|ExecutionSequence`
    (:`then_0`
      ;[1 1 1] Make sure the ledge is at the right hight (Can change with Min and Max vault height)
      (if (not (`KismetMathLibrary.InRange_FloatFloat` (- (.z _hit_location_2) (.z _hit_traceend)) (`self.MinVaultHeight`) (`self.MaxVaultHeight`)))
        (return false (0.0 0.0 0.0))))
    (:`then_1`
      ;[1 1 1] Make sure the area we are vaulting to is walkable
      (if (< (.z _hit_normal_2) (`CharacterMovementComponent.K2_GetWalkableFloorZ` (`Character.CharacterMovement` (`self.Player`))))
        (return false (0.0 0.0 0.0))))
    (:`then_2`
      ;[1 1 1] Makes Sure No object is Vauliting area that would obscure player
      (bind _output_get (set `local.EndPosition_Local` (+ _hit_location (`KismetMathLibrary.MakeVector` 0.0 0.0 (`CapsuleComponent.GetScaledCapsuleHalfHeight` (`local.Capsule`))))))
      (bind _resault (`self.CheckCapsuleCollision` (+ _output_get (`KismetMathLibrary.MakeVector` 0.0 0.0 _returnvalue)) (`CapsuleComponent.GetScaledCapsuleHalfHeight` _capsule) _returnvalue))
      (if _resault
        (return false (0.0 0.0 0.0))))
    (:`then_3`
      (return true (`local.EndPosition_Local`)))))

(fn `CheckCapsuleCollision`
  (params (CapCenter :type "Vector Structure") (CapHalfHeight :type "Float (double-precision)") (CapRadius :type "Float (double-precision)") (DrawDebug :type Boolean))
  (returns (Resault :type Boolean))
  (`|ExecutionSequence`
    (:`then_0`
      (if (`local.DrawDebug`)
        _))
    (:`then_1`
      (bind (_outactors _returnvalue) (`KismetSystemLibrary.CapsuleOverlapActors` (`local.CapCenter`) (`local.CapRadius`) (`local.CapHalfHeight`) (`|MakeArray` "ObjectTypeQuery1" "ObjectTypeQuery2" "ObjectTypeQuery3" "ObjectTypeQuery4" "ObjectTypeQuery5" "ObjectTypeQuery6" :!type "EObjectTypeQuery Enum") null (`|MakeArray` (`self.Player`) :!type "Actor Object Reference")))
      (return _returnvalue))))

(fn `GetVaultingState`
  (returns (VaultState :type "/Game/Blueprints/Player_BP/EVaultingState Enum"))
  (return (`self.VaultState`)))

(fn `Tick Vault`
  (params (DeltaSeconds :type "Float (double-precision)"))
  (`|ExecutionSequence`
    (:`then_0`
      (set `self.VaultProgress` (`KismetMathLibrary.FClamp` (+ (`self.VaultProgress`) (/ (`local.DeltaSeconds`) (`self.VaultSpeed`)))))
      (`Actor.K2_SetActorLocation` (`self.Player`) (`KismetMathLibrary.VLerp` (`self.StartPosition`) (`self.EndPosition`) (`self.VaultProgress`)) false true))
    (:`then_1`
      (if (>= (`self.VaultProgress`) 1.0)
        (set `self.VaultState` "NewEnumerator0")))))