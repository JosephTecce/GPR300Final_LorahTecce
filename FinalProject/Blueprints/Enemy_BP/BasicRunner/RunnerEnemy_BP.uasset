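; RunnerEnemy_BP is a runner enemy that damages the player on contact and destroys itself when its health runs out.
; On hit, it messages any actor implementing the RunnerCollide interface, passing itself.
; Its CollidedwithPlayer event subtracts damage from a non-invincible player, sets the player invincible and triggers the damage effect.
; TookDamage only checks current health, which starts at max on BeginPlay, and destroys the actor at zero or below.
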(event `self.ReceiveBeginPlay`
  (set `self.CurrentHealth` (`self.MaxHealth`)))

(event `/Game/Blueprints/Player_BP/PlayerCollide_Inter.CollidedWithPlayer`
  (params (Player :type "/Game/FirstPersonBP/Blueprints/FirstPersonCharacter Object Reference"))
  (if (not (`/Game/FirstPersonBP/Blueprints/FirstPersonCharacter.IsInvinsible` Player))
    (set `/Game/FirstPersonBP/Blueprints/FirstPersonCharacter.CurHealth` (- (`/Game/FirstPersonBP/Blueprints/FirstPersonCharacter.CurHealth` Player) (`self.Damage`)) Player)
    (set `/Game/FirstPersonBP/Blueprints/FirstPersonCharacter.IsInvinsible` true Player)
    (`/Game/FirstPersonBP/Blueprints/FirstPersonCharacter.DamageEffect` Player)))

(event `self.ReceiveHit`
  (params (MyComp :type "PrimitiveComponent Object Reference") (Other :type "Actor Object Reference") (OtherComp :type "PrimitiveComponent Object Reference") (bSelfMoved :type Boolean) (HitLocation :type "Vector Structure") (HitNormal :type "Vector Structure") (NormalImpulse :type "Vector Structure") (Hit :type "HitResult Structure (by ref)"))
  (if (`KismetSystemLibrary.DoesImplementInterface` Other "/Game/Blueprints/Enemy_BP/BasicRunner/RunnerCollide_Inst.RunnerCollide_Inst_C")
    (message `/Game/Blueprints/Enemy_BP/BasicRunner/RunnerCollide_Inst.CollidedWithRunner` Other self)))

(event `TookDamage`
  (if (<= (`self.CurrentHealth`) 0.0)
    (`self.K2_DestroyActor`)))

(fn `UserConstructionScript`)